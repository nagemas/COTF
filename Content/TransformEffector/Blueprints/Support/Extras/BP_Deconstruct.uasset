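; BP_Deconstruct is a utility actor that breaks a referenced Blueprint actor into individual StaticMeshActors.
; Its Deconstruct function walks all descendants of the target's root component and casts each to a static mesh component.
; For each mesh, it spawns an actor at the same world transform, copies the mesh and materials, and prints the component name.
; The source actor stays untouched, and the event graph is empty.
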(fn `Deconstruct`
  (for _array_element (`SceneComponent.GetChildrenComponents` (`Actor.RootComponent` (`self.Blueprint for deconstruction`)) true)
    (bind _asstatic_mesh_component (cast `StaticMeshComponent` _array_element))
    (set `self.MyLoopComponent` _asstatic_mesh_component)
    (bind _returnvalue (`|SpawnActorFromClass` "/Script/Engine.StaticMeshActor" (`SceneComponent.K2_GetComponentToWorld` _asstatic_mesh_component) "Undefined" "OverrideRootScale" null null))
    (bind _staticmeshcomponent (`StaticMeshActor.StaticMeshComponent` _returnvalue))
    (`StaticMeshComponent.SetStaticMesh` _staticmeshcomponent (`StaticMeshComponent.StaticMesh` _asstatic_mesh_component))
    (`KismetSystemLibrary.PrintString` (`KismetSystemLibrary.GetObjectName` _asstatic_mesh_component))
    (for (_array_element_2 _array_index) (`MeshComponent.GetMaterials` (`self.MyLoopComponent`))
      (`PrimitiveComponent.SetMaterial` _staticmeshcomponent _array_index _array_element_2))))

(fn `UserConstructionScript`)