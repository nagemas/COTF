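; BP_SinMovement is an actor that bobs vertically along a sine wave around its starting position.
; BeginPlay stores the starting location; while the ONOFF flag is set, Tick offsets only Z using game time, Speed and Distance.
; The offset comes from a math expression fed negative half Distance as amplitude, moving the root component directly.
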(event EventBeginPlay
  (Variables|Default|SetDefaultLocation (Transformation|GetActorLocation)))

(event Collision|EventActorBeginOverlap
  (params (OtherActor :type Actor%20Object%20Reference)))

(event EventTick
  (params (DeltaSeconds :type Float%20%28single-precision%29))
  (bind _defaultlocation (Variables|Default|GetDefaultLocation))
  (if (Variables|Default|GetON/OFF)
    (Transformation|SetWorldLocation (Variables|Default|GetDefaultSceneRoot) (Math|Vector|MakeVector (.x _defaultlocation) (.y _defaultlocation) (+ (.z _defaultlocation) (|(((Sin((time*spd)))+1)*dist) (Utilities|Time|GetGameTimeinSeconds) (Variables|Default|GetSpeed) (* -1 (/ (Variables|Default|GetDistance) 2.0))))) false false)))

(fn ConstructionScript)