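; A trigger-box actor that acts as an external reset input for the TransformEffector solver.
; On start it shows a red material and, after a short delay, caches the first BP_TE_Solver in the level, retrying on Tick while that reference is invalid.
; Overlapping the box turns it green and calls the solver's ResetToDefaultTransformation; ending the overlap turns it red again.
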(event `self.ReceiveBeginPlay`
  (`PrimitiveComponent.SetMaterial` (`self.StaticMeshComponent`) 0 "/Game/TransformEffector/Materials/MI_Red.MI_Red")
  (`KismetSystemLibrary.Delay` 0.2)
  (bind _outactors (`GameplayStatics.GetAllActorsOfClass` "/Game/TransformEffector/Blueprints/Support/Solvers/BP_TE_Solver.BP_TE_Solver_C" :!label _label))
  (set `self.Solver` (`|GetArrayItem` _outactors)))

(event `self.ReceiveTick`
  (params (DeltaSeconds :type "Float (single-precision)"))
  (`/Engine/EditorBlueprintResources/StandardMacros.IsValid` (`self.Solver`)
    (:`Is Not Valid`
      (goto _label))))

(event `self.Box.OnComponentBeginOverlap`
  (params (OverlappedComponent :type "PrimitiveComponent Object Reference") (OtherActor :type "Actor Object Reference") (OtherComp :type "PrimitiveComponent Object Reference") (OtherBodyIndex :type Integer) (bFromSweep :type Boolean) (SweepResult :type "HitResult Structure (by ref)"))
  (`PrimitiveComponent.SetMaterial` (`self.StaticMeshComponent`) 0 "/Game/TransformEffector/Materials/MI_Green02.MI_Green02")
  (`/Game/TransformEffector/Blueprints/Support/Solvers/BP_TE_Solver.Reset to Default Transformation` (`self.Solver`)))

(event `self.Box.OnComponentEndOverlap`
  (params (OverlappedComponent :type "PrimitiveComponent Object Reference") (OtherActor :type "Actor Object Reference") (OtherComp :type "PrimitiveComponent Object Reference") (OtherBodyIndex :type Integer))
  (`PrimitiveComponent.SetMaterial` (`self.StaticMeshComponent`) 0 "/Game/TransformEffector/Materials/MI_Red.MI_Red"))

(fn `UserConstructionScript`)