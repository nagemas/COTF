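; BP_ExternalInput_ON_OFF is a trigger actor that switches a referenced TransformEffector on and off.
; Entering its Box sets the effector's ONOFF flag true and turns the mesh material green; leaving sets it false and turns the mesh red.
; A separate actor-level begin-overlap event also sets the red material, without touching the flag.
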(event `self.ReceiveActorBeginOverlap`
  (params (OtherActor :type "Actor Object Reference"))
  (`PrimitiveComponent.SetMaterial` (`self.StaticMeshComponent`) 0 "/Game/TransformEffector/Materials/MI_Red.MI_Red"))

(event `self.Box.OnComponentBeginOverlap`
  (params (OverlappedComponent :type "PrimitiveComponent Object Reference") (OtherActor :type "Actor Object Reference") (OtherComp :type "PrimitiveComponent Object Reference") (OtherBodyIndex :type Integer) (bFromSweep :type Boolean) (SweepResult :type "HitResult Structure (by ref)"))
  (`PrimitiveComponent.SetMaterial` (`self.StaticMeshComponent`) 0 "/Game/TransformEffector/Materials/MI_Green02.MI_Green02")
  (set `/Game/TransformEffector/Blueprints/Support/Solvers/BP_Transform_Effector_V2.ON/OFF` true (`self.Transform Effector`)))

(event `self.Box.OnComponentEndOverlap`
  (params (OverlappedComponent :type "PrimitiveComponent Object Reference") (OtherActor :type "Actor Object Reference") (OtherComp :type "PrimitiveComponent Object Reference") (OtherBodyIndex :type Integer))
  (`PrimitiveComponent.SetMaterial` (`self.StaticMeshComponent`) 0 "/Game/TransformEffector/Materials/MI_Red.MI_Red")
  (set `/Game/TransformEffector/Blueprints/Support/Solvers/BP_Transform_Effector_V2.ON/OFF` false (`self.Transform Effector`)))

(fn `UserConstructionScript`)