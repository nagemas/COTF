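; Transform effector actor that carries a tag, priority and min/max distance range, shown by helper spheres and text with optional in-game visibility.
; On BeginPlay the highest-priority effector spawns a BP_TE_Solver and destroys duplicates, keeping one shared solver.
; Tick finds that solver if unset, otherwise updates IsBPMoving.
; The flag is briefly forced on at startup, then compares last-frame location when UpdateOnlyWhenMoving is set.
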(event `self.ReceiveBeginPlay`
  (`self.Get Priority`))

(event `self.ReceiveTick`
  (params (DeltaSeconds :type "Float (single-precision)"))
  ;[0 0 0] Set priority collector reference
  (`/Engine/EditorBlueprintResources/StandardMacros.IsValid` (`self.TE Solver`)
    (:`Is Valid`
      (`self.Is BP Moving?`))
    (:`Is Not Valid`
      (bind _outactors (`GameplayStatics.GetAllActorsOfClass` "/Game/TransformEffector/Blueprints/Support/Solvers/BP_TE_Solver.BP_TE_Solver_C"))
      (set `self.TE Solver` (`|GetArrayItem` _outactors)))))

(fn `UserConstructionScript`
  (bind _spheremax (`self.SphereMax`))
  (bind _helpertextscale (`self.HelperTextScale`))
  (`|ExecutionSequence`
    (:`then_0`
      ;[0.1562 0.1562 0.1562] Set scale of helper spheres
      (`SceneComponent.SetWorldScale3D` (`self.SphereMin`) (`KismetMathLibrary.Conv_DoubleToVector` (`self.Distance Min`)))
      (`SceneComponent.SetWorldScale3D` (`self.SphereMax`) (`KismetMathLibrary.Conv_DoubleToVector` (`self.Distance Max`)))
      ;[0.1562 0.1562 0.1562] Set helper spheres visibility
      (if (`self.Helpers Visible in Game`)
        (`SceneComponent.SetHiddenInGame` _spheremax false false)
        (`SceneComponent.SetHiddenInGame` (`self.SphereMin`) false false)
        (`SceneComponent.SetHiddenInGame` (`self.Billboard`) false false)
        (`SceneComponent.SetHiddenInGame` (`self.TagText`) false false)
        (`SceneComponent.SetHiddenInGame` (`self.PriorityText`) false false)
        (else
          (`SceneComponent.SetHiddenInGame` _spheremax true false)
          (`SceneComponent.SetHiddenInGame` (`self.SphereMin`) true false)
          (`SceneComponent.SetHiddenInGame` (`self.Billboard`) true false)
          (`SceneComponent.SetHiddenInGame` (`self.PriorityText`) true false)
          (`SceneComponent.SetHiddenInGame` (`self.TagText`) true false))))
    (:`then_1`
      ;[0.1562 0.1562 0.1562] Set Tag and Priority text to print
      (`TextRenderComponent.K2_SetText` (`self.TagText`) (`KismetTextLibrary.Conv_NameToText` (`self.EffectorTag`)))
      (`TextRenderComponent.K2_SetText` (`self.PriorityText`) (`KismetTextLibrary.Conv_IntToText` (`self.Priority`))))
    (:`then_2`
      ;[0.1562 0.1562 0.1562] Set Tag and priority text size
      (`SceneComponent.SetWorldScale3D` (`self.PriorityText`) (`KismetMathLibrary.MakeVector` _helpertextscale _helpertextscale _helpertextscale)))))